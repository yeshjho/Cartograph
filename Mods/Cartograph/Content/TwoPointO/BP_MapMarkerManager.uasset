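; BP_MapMarkerManager is an actor that draws map markers as instanced static meshes and renders them through a scene capture.
; On BeginPlay it adds one large, rotated instance below the origin and styles it through per-instance custom data.
; The 2D map capture's show-only list is then limited to the actor's own components, and the scene is captured once rather than through any update logic.
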(event `self.ReceiveBeginPlay`
  (bind _mapcapturecomponent2d (`self.MapCaptureComponent2D`))
  (bind _instancedstaticmesh (`self.InstancedStaticMesh`))
  (`|ExecutionSequence`
    (:`then_0`
      (`self.SetOwner` self))
    (:`then_1`
      (bind _returnvalue (`InstancedStaticMeshComponent.AddInstance` _instancedstaticmesh (`KismetMathLibrary.MakeTransform` (0.0 0.0 -3500.0) (struct :`Pitch` 45.0 :`Yaw` 45.0) (1000.0 1000.0 1000.0)) false))
      (`InstancedStaticMeshComponent.SetCustomDataValue` _instancedstaticmesh _returnvalue 0 1.0 false)
      (`InstancedStaticMeshComponent.SetCustomDataValue` _instancedstaticmesh _returnvalue 1 0.0 false)
      (`InstancedStaticMeshComponent.SetCustomDataValue` _instancedstaticmesh _returnvalue 2 1.0 false)
      (`InstancedStaticMeshComponent.SetCustomDataValue` _instancedstaticmesh _returnvalue 6 0.8 true))
    (:`then_2`
      (`SceneCaptureComponent.ClearShowOnlyComponents` _mapcapturecomponent2d)
      (`SceneCaptureComponent.ShowOnlyActorComponents` _mapcapturecomponent2d self false)
      (`SceneCaptureComponent2D.CaptureScene` _mapcapturecomponent2d))))

(fn `UserConstructionScript`)